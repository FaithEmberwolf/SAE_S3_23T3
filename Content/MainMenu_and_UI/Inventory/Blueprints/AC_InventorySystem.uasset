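; Inventory component that holds a fixed-size array of item slots and handles look-at detection and pickup interaction.
; A per-tick sphere trace tracks the looked-at actor, whose AC_ItemData receives the pickup input.
; AddToInventory adds units singly using DT_ItemData stack limits, but FindSlot never reports success and stack writes index by Quantity.
; RemoveFromInventory is an empty stub, and key 2 prints contents for debugging.
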(event Input|EnhancedActionEvents|EnhancedInputActionIA_PickUp
  (params (ActionValue :type Boolean) (ElapsedSeconds :type Float%20%28double-precision%29) (TriggeredSeconds :type Float%20%28double-precision%29) (InputAction :type Input%20Action%20Object%20Reference :default "/Game/ThirdPerson/Input/Actions/IA_PickUp.IA_PickUp"))
  (:Started
    (Class|IInteractionInterface|Interactwith(Message) (Actor|GetComponentbyClass (Variables|Default|GetLookAtActor) "/Game/MainMenu_and_UI/Inventory/Blueprints/AC_ItemData.AC_ItemData_C") (.AsBP%20Third%20Person%20Character (Utilities|Casting|CastToBP_ThirdPersonCharacter (Components|GetOwner))))))

(event EventTick
  (params (DeltaSeconds :type Float%20%28single-precision%29))
  (CallFunction|InteractionTracing))

(event EventBeginPlay
  (Utilities|Array|Resize (Variables|Default|GetInventoryContent) (Variables|Default|GetInventorySize)))

(event Input|KeyboardEvents|2
  (params (Key :type Key%20Structure :default "None"))
  (:Pressed
    (CallFunction|DEBUGPrintContents)))

(fn AddtoInventory
  (params (ItemID :type Name) (Quantity :type Integer))
  (LocalVariables|SetLocalQuantityRemaining Quantity)
  (while (and (> (LocalVariables|GetLocalQuantityRemaining) 0) (not (LocalVariables|GetLocalHasFailed)))
    (bind (_index _foundslot) (CallFunction|FindSlot ItemID))
    (if _foundslot
      ;[1 1 1] Found slot with space
      (CallFunction|AddtoStack _index 1)
      (Math|Integer|DecrementInt (LocalVariables|GetLocalQuantityRemaining))
      (else
        ;[1 1 1] Look for empty slot
        (if (CallFunction|AnyEmptySlots)
          (bind _success (CallFunction|CreateNewStack ItemID 1))
          (if _success
            (Math|Integer|DecrementInt (LocalVariables|GetLocalQuantityRemaining))
            (else
              (LocalVariables|SetLocalHasFailed true)))
          (else
            (LocalVariables|SetLocalHasFailed true))))))
  (return (not (LocalVariables|GetLocalHasFailed)) (LocalVariables|GetLocalQuantityRemaining)))

(fn FindSlot
  (params (ItemID :type Name))
  (for (_array_element _array_index) (Variables|Default|GetInventoryContent)
    (if (== (.ItemID (Utilities|Struct|BreakF_SlotStruct _array_element)) ItemID)
      (if (< (.Quantity (Utilities|Struct|BreakF_SlotStruct _array_element)) (CallFunction|GetMaxStackSize ItemID))
        (return _array_index false))))
  (return -1 false))

(fn GetMaxStackSize
  (params (RowName :type Name))
  (bind _returnvalue (Utilities|GetDataTableRow "/Game/MainMenu_and_UI/Inventory/Blueprints/DT_ItemData.DT_ItemData" RowName)
    (:then
      (return (Utilities|Struct|BreakF_ItemStruct _returnvalue)))
    (:RowNotFound
      (return -1))))

(fn AddtoStack
  (params (Index :type Integer) (Quantity :type Integer))
  (bind _inventorycontent (Variables|Default|GetInventoryContent))
  (bind _output (Utilities|Array|Get(acopy) _inventorycontent Quantity))
  (Utilities|Array|SetArrayElem (Variables|Default|GetInventoryContent) Index (Utilities|Struct|MakeF_SlotStruct (.itemid _output) (.quantity _output))))

(fn AnyEmptySlots
  (for _array_element (Variables|Default|GetInventoryContent)
    (if (== (.Quantity (Utilities|Struct|BreakF_SlotStruct _array_element)) 0)
      (return true)))
  (return false))

(fn CreateNewStack
  (params (ItemID :type Name) (Quantity :type Integer))
  (if (CallFunction|AnyEmptySlots)
    (Utilities|Array|SetArrayElem (Variables|Default|GetInventoryContent) Quantity (Utilities|Struct|MakeF_SlotStruct ItemID Quantity))
    (return true)
    (else
      (return false))))

(fn InteractionTracing
  (bind _returnvalue (Game|GetPlayerCameraManager 0))
  (bind (_outhit _returnvalue_2) (Collision|SphereTraceByChannel "0, 0, 0" (+ (Transformation|GetActorLocation _returnvalue) (* (Transformation|GetActorForwardVector _returnvalue) (Variables|Default|GetInteractionRange))) 0.0 "TraceTypeQuery3" false (Utilities|Array|MakeArray (Components|GetOwner)) "None"))
  (if _returnvalue_2
    (if (!= (.HitActor (Collision|BreakHitResult _outhit)) (Variables|Default|GetLookAtActor))
      (bind _output_get (Variables|Default|SetLookAtActor (.HitActor (Collision|BreakHitResult _outhit))))
      (bind _message (Class|IInteractionInterface|Lookat(Message) _output_get))
      (Development|PrintString (Utilities|String|ToString(Text) _message)))
    (else
      (Variables|Default|SetLookAtActor 0))))

(fn RemovefromInventory)

(fn DEBUGPrintContents
  (for (_array_element _array_index) (Variables|Default|GetInventoryContent)
    (Development|PrintString (Utilities|String|Append (Utilities|String|ToString(Integer) _array_index) " ; " (Utilities|String|ToString(Name) (.ItemID (Utilities|Struct|BreakF_SlotStruct _array_element))) " = " (Utilities|String|ToString(Integer) (.Quantity (Utilities|Struct|BreakF_SlotStruct _array_element)))))))