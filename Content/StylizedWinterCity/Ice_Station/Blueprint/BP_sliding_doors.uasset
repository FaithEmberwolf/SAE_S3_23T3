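; Sliding door actor for the Ice Station that opens when something enters its trigger box and closes when it leaves.
; Box overlap events play and reverse the Slide timeline.
; Each timeline update lerps the relative locations of the top and bottom door meshes between stored closed and open vectors, without sweeping.
; Overlaps are not filtered, so any overlapping actor drives the door.
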(event OnComponentBeginOverlap(Box)
  (params (OverlappedComponent :type Primitive%20Component%20Object%20Reference) (OtherActor :type Actor%20Object%20Reference) (OtherComp :type Primitive%20Component%20Object%20Reference) (OtherBodyIndex :type Integer) (bFromSweep :type Boolean) (SweepResult :type Hit%20Result%20Structure%20%28by%20ref%29))
  ;[1 1 1] Door sliding
  (bind _newtrack_0 (Timeline|Slide Play)
    (:Update
      ;[1 1 1] New location door top
      (Transformation|SetRelativeLocation (Variables|Default|GetSM_door_top) (Math|Vector|Lerp(Vector) (Variables|Default|Getcurrent_location) (Variables|Default|Getnew_location) _newtrack_0) false false)
      (Transformation|SetRelativeLocation (Variables|Default|GetSM_door_bottom) (Math|Vector|Lerp(Vector) (Variables|Default|GetCurrent%20Location%20Bottom) (Variables|Default|GetNew%20Location%20Bottom) _newtrack_0) false false))))

(event OnComponentEndOverlap(Box)
  (params (OverlappedComponent :type Primitive%20Component%20Object%20Reference) (OtherActor :type Actor%20Object%20Reference) (OtherComp :type Primitive%20Component%20Object%20Reference) (OtherBodyIndex :type Integer))
  ;[1 1 1] Door sliding
  (bind _newtrack_0 (Timeline|Slide Reverse)
    (:Update
      ;[1 1 1] New location door top
      (Transformation|SetRelativeLocation (Variables|Default|GetSM_door_top) (Math|Vector|Lerp(Vector) (Variables|Default|Getcurrent_location) (Variables|Default|Getnew_location) _newtrack_0) false false)
      (Transformation|SetRelativeLocation (Variables|Default|GetSM_door_bottom) (Math|Vector|Lerp(Vector) (Variables|Default|GetCurrent%20Location%20Bottom) (Variables|Default|GetNew%20Location%20Bottom) _newtrack_0) false false))))

(fn ConstructionScript)