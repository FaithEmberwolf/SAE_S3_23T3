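; BP_Train is an interactive train actor that the player moves along a straight path and that has sliding doors.
; A character inside Box enables input on the actor, so E plays and Q reverses a timeline that lerps the train's relative location between StartPoint and EndPoint.
; Any overlap with Box1 plays a second timeline that slides both doors open by lerping their positions, and leaving reverses it.
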(event OnComponentBeginOverlap(Box)
  (params (OverlappedComponent :type Primitive%20Component%20Object%20Reference) (OtherActor :type Actor%20Object%20Reference) (OtherComp :type Primitive%20Component%20Object%20Reference) (OtherBodyIndex :type Integer) (bFromSweep :type Boolean) (SweepResult :type Hit%20Result%20Structure%20%28by%20ref%29))
  (Utilities|Casting|CastToCharacter OtherActor)
  (Input|EnableInput (Game|GetPlayerController 0)))

(event OnComponentEndOverlap(Box)
  (params (OverlappedComponent :type Primitive%20Component%20Object%20Reference) (OtherActor :type Actor%20Object%20Reference) (OtherComp :type Primitive%20Component%20Object%20Reference) (OtherBodyIndex :type Integer))
  (Utilities|Casting|CastToCharacter OtherActor)
  (Input|DisableInput (Game|GetPlayerController 0)))

(event OnComponentBeginOverlap(Box1)
  (params (OverlappedComponent :type Primitive%20Component%20Object%20Reference) (OtherActor :type Actor%20Object%20Reference) (OtherComp :type Primitive%20Component%20Object%20Reference) (OtherBodyIndex :type Integer) (bFromSweep :type Boolean) (SweepResult :type Hit%20Result%20Structure%20%28by%20ref%29))
  ;[1 1 1] Door sliding
  (bind _newtrack_0 (Timeline|Timeline_0 Play)
    (:Update
      ;[1 1 1] New location door Right
      (Transformation|SetRelativeLocation (Variables|Default|GetDoor_R) (Math|Vector|Lerp(Vector) (Variables|Default|Getcurrent_location_R) (Variables|Default|Getnew_location_R) _newtrack_0) false false)
      ;[1 1 1] Door Left
      (Transformation|SetRelativeLocation (Variables|Default|GetDoor_L) (Math|Vector|Lerp(Vector) (Variables|Default|GetCurrent%20Location_L) (Variables|Default|GetNew%20Location_L) _newtrack_0) false false))))

(event OnComponentEndOverlap(Box1)
  (params (OverlappedComponent :type Primitive%20Component%20Object%20Reference) (OtherActor :type Actor%20Object%20Reference) (OtherComp :type Primitive%20Component%20Object%20Reference) (OtherBodyIndex :type Integer))
  ;[1 1 1] Door sliding
  (bind _newtrack_0 (Timeline|Timeline_0 Reverse)
    (:Update
      ;[1 1 1] New location door Right
      (Transformation|SetRelativeLocation (Variables|Default|GetDoor_R) (Math|Vector|Lerp(Vector) (Variables|Default|Getcurrent_location_R) (Variables|Default|Getnew_location_R) _newtrack_0) false false)
      ;[1 1 1] Door Left
      (Transformation|SetRelativeLocation (Variables|Default|GetDoor_L) (Math|Vector|Lerp(Vector) (Variables|Default|GetCurrent%20Location_L) (Variables|Default|GetNew%20Location_L) _newtrack_0) false false))))

(event Input|KeyboardEvents|Q
  (params (Key :type Key%20Structure))
  (:Pressed
    (bind _newtrack_0 (Timeline|Timeline_1 Reverse)
      (:Update
        (Transformation|SetRelativeLocation (Variables|Default|GetTrain) (Math|Vector|Lerp(Vector) (Variables|Default|GetStart%20point) (Variables|Default|GetEnd%20point) _newtrack_0) false false)))))

(event Input|KeyboardEvents|E
  (params (Key :type Key%20Structure))
  (:Pressed
    (bind _newtrack_0 (Timeline|Timeline_1 Play)
      (:Update
        (Transformation|SetRelativeLocation (Variables|Default|GetTrain) (Math|Vector|Lerp(Vector) (Variables|Default|GetStart%20point) (Variables|Default|GetEnd%20point) _newtrack_0) false false)))))

(fn ConstructionScript)