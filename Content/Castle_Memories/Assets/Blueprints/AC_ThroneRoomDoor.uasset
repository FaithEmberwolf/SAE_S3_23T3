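; Throne room door component that removes its owning actor when the player interacts while holding the required item.
; Interactwith checks the player's inventory component and compares the RowName of the ItemID variable to the item at index 1 of InventoryContent only.
; A match destroys the owner outright, without consuming the item, and LookAt returns an empty string, so it supplies no prompt text.
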(event EventInteractwith
  (params (PlayerCharacter :type BP%20Third%20Person%20Character%20Object%20Reference))
  (bind _ac_inventorysystem (Variables|/Game/ThirdPerson/Blueprints/BP_ThirdPersonCharacter.BP_ThirdPersonCharacter_C|GetAC_InventorySystem PlayerCharacter))
  (Utilities|IsValid _ac_inventorysystem
    (:Is%20Valid
      (if (== (.rowname (Variables|Default|GetItemID)) (.itemid (Utilities|Array|Get(acopy) (Variables|/Game/MainMenu_and_UI/Inventory/Blueprints/AC_InventorySystem.AC_InventorySystem_C|GetInventoryContent _ac_inventorysystem) 1)))
        (Actor|DestroyActor (Components|GetOwner))))))

(fn Lookat
  (return ""))