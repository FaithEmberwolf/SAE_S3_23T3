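; Inventory component that holds item slots and handles the owner's interaction with world objects.
; Each tick a camera-forward sphere trace caches the looked-at actor and prints its message; Interact sends it an interact message.
; AddToInventory is written to stack units using DT_ItemData limits or open new slots.
; FindSlot never reports a match, slot writes use Quantity as an index, and RemoveFromInventory is empty.
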(event Custom|Object_Interact
  (params (Target :type Actor%20Object%20Reference))
  (bind _returnvalue (Actor|GetComponentbyClass Target "/Game/Castle_Memories/Assets/Blueprints/Inventory/AC_ItemDataComponent.AC_ItemDataComponent_C"))
  (Utilities|IsValid _returnvalue
    (:Is%20Valid
      (Class|IInteractInterface|Interactwith(Message) _returnvalue (.AsBP%20DEF%20Third%20Person%20Swapper%20Neon%20Dash (Utilities|Casting|CastToBP_DEF_ThirdPerson_Swapper_NeonDash (Components|GetOwner)))))))

(event EventTick
  (params (DeltaSeconds :type Float%20%28single-precision%29))
  (CallFunction|InteractionTrace))

(event EventBeginPlay
  (Utilities|Array|Resize (Variables|Default|GetContent) (Variables|Default|GetInventorySize)))

(event Input|ActionEvents|InputActionInteract
  (params (Key :type Key%20Structure :default "None"))
  (:Pressed
    (bind _lookatactor (Variables|Default|GetLookATActor)
      (:then
        (CallFunction|ObjectInteract _lookatactor)
        (bind _lookatactor_2 (Variables|Default|GetLookATActor)
          (:then
            (Class|IInteractInterface|Interactwith(Message) _lookatactor_2 (.AsBP%20DEF%20Third%20Person%20Swapper%20Neon%20Dash (Utilities|Casting|CastToBP_DEF_ThirdPerson_Swapper_NeonDash (Components|GetOwner)))))
          (:else)))
      (:else))))

(event Input|KeyboardEvents|NumPadOne
  (params (Key :type Key%20Structure :default "None"))
  (:Pressed
    (CallFunction|DEBUGPrintContent)))

(fn AddtoInventory
  (params (ItemID :type Name) (Quantity :type Integer))
  (LocalVariables|SetLocal_QuantityRemaining Quantity)
  (while (and (> (LocalVariables|GetLocal_QuantityRemaining) 0) (not (LocalVariables|GetLocal_HasFailed)))
    (bind (_index _foundslot) (CallFunction|FindSlot ItemID))
    (if _foundslot
      (CallFunction|AddtoStack _index 1)
      (Math|Integer|DecrementInt (LocalVariables|GetLocal_QuantityRemaining))
      (elif (.HasEmptySlot (CallFunction|AnyEmptySlotsAvalible))
        (bind _success (CallFunction|CreateNewStack ItemID 1))
        (if _success
          (Math|Integer|DecrementInt (LocalVariables|GetLocal_QuantityRemaining))
          (else
            (LocalVariables|SetLocal_HasFailed true))))))
  (return (not (LocalVariables|GetLocal_HasFailed)) (LocalVariables|GetLocal_QuantityRemaining)))

(fn RemovefromInventory)

(fn InteractionTrace
  (bind _returnvalue (Game|GetPlayerCameraManager 0))
  (bind _returnvalue_2 (Transformation|GetActorLocation _returnvalue))
  (bind (_outhit _returnvalue_3) (Collision|SphereTraceByChannel _returnvalue_2 (+ _returnvalue_2 (* (Transformation|GetActorForwardVector _returnvalue) (Variables|Default|GetInteraction%20Range))) 15.0 "TraceTypeQuery4" false (Utilities|Array|MakeArray (Components|GetOwner)) "None"))
  (if _returnvalue_3
    (if (!= (.HitActor (Collision|BreakHitResult _outhit)) (Variables|Default|GetLookATActor))
      (bind _output_get (Variables|Default|SetLookATActor (.HitActor (Collision|BreakHitResult _outhit))))
      (bind _message (Class|IInteractInterface|Lookat(Message) _output_get))
      (Development|PrintString (Utilities|String|ToString(Text) _message)))
    (else
      (Variables|Default|SetLookATActor 0))))

(fn FindSlot
  (params (ItemID :type Name))
  (for (_array_element _array_index) (Variables|Default|GetContent)
    (if (== (.ItemID (Utilities|Struct|BreakF_SlotStrut _array_element)) ItemID)
      (if (< (.Quantity (Utilities|Struct|BreakF_SlotStrut _array_element)) (CallFunction|GetMaxStackSize ItemID))
        (return _array_index false))))
  (return -1 false))

(fn GetMaxStackSize
  (params (ItemID :type Name))
  (bind _returnvalue (Utilities|GetDataTableRow "/Game/Castle_Memories/Assets/Blueprints/Inventory/DT_ItemData.DT_ItemData" ItemID)
    (:then
      (return (.StackSize (Utilities|Struct|BreakF_ItemStrut _returnvalue))))
    (:RowNotFound
      (return -1))))

(fn AddtoStack
  (params (Index :type Integer) (Quantity :type Integer))
  (bind _content (Variables|Default|GetContent))
  (bind _output (Utilities|Array|Get(acopy) _content Quantity))
  (Utilities|Array|SetArrayElem (Variables|Default|GetContent) Index (Utilities|Struct|MakeF_SlotStrut (.itemid _output) (+ (.quantity _output) Quantity))))

(fn AnyEmptySlotsAvalible
  (for (_array_element _array_index) (Variables|Default|GetContent)
    (if (== (.Quantity (Utilities|Struct|BreakF_SlotStrut _array_element)) 0)
      (return true _array_index)))
  (return false -1))

(fn CreateNewStack
  (params (ItemID :type Name) (Quantity :type Integer))
  (if (.HasEmptySlot (CallFunction|AnyEmptySlotsAvalible))
    (Utilities|Array|SetArrayElem (Variables|Default|GetContent) Quantity (Utilities|Struct|MakeF_SlotStrut ItemID Quantity))
    (return true)
    (else
      (return false))))

(fn DEBUGPrintContent
  (for (_array_element _array_index) (Variables|Default|GetContent)
    (Development|PrintString (Utilities|String|Append (Utilities|String|ToString(Integer) _array_index) "; " (Utilities|String|ToString(Name) (.ItemID (Utilities|Struct|BreakF_SlotStrut _array_element))) " = " (Utilities|String|ToString(Integer) (.Quantity (Utilities|Struct|BreakF_SlotStrut _array_element)))))))